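; DefaultCharacter is a first-person player character with movement, mouse look, lives, projectile firing from the camera, and win and fail outcomes.
; On BeginPlay it takes lives from UserGameMode, creates the UI widget and stores its start location for teleport resets.
; Losing a life at zero triggers PlayerFail, which, like PlayerWin, resets lives and timer and shows its screen.
; Slowdown temporarily halves walk speed with an on-screen alert.
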(event Custom|Slowdown
  (bind _widgetref (Variables|Default|GetWidgetRef))
  (bind _charactermovement (Variables|Character|GetCharacterMovement))
  (bind _charactermovement_2 (Variables|Character|GetCharacterMovement))
  (Variables|/Script/Engine.CharacterMovementComponent|SetMaxWalkSpeed _charactermovement (/ (Variables|/Script/Engine.CharacterMovementComponent|GetMaxWalkSpeed _charactermovement) 2.0))
  (Default|ShowHideSlowdownAlertF _widgetref true)
  (Utilities|FlowControl|Delay 1.5)
  (Default|ShowHideSlowdownAlertF _widgetref false)
  (Variables|/Script/Engine.CharacterMovementComponent|SetMaxWalkSpeed _charactermovement_2 (* (Variables|/Script/Engine.CharacterMovementComponent|GetMaxWalkSpeed _charactermovement_2) 2.0)))

(event Custom|PlayerFail
  (bind _widgetref (Variables|Default|GetWidgetRef))
  (CallFunction|SetDefaultLivesF)
  (Default|ShowHideFailScreenF _widgetref true)
  (Default|FocusPlayerControleronUiorGameF _widgetref true)
  (Default|SetDefaultLivesF _widgetref)
  (Default|SetDefaultTimerF _widgetref)
  (Default|ClearTimerF _widgetref))

(event Custom|PlayerWin
  (bind _widgetref (Variables|Default|GetWidgetRef))
  (CallFunction|SetDefaultLivesF)
  (Default|ShowHideWonScreenF _widgetref true)
  (Default|FocusPlayerControleronUiorGameF _widgetref true)
  (Default|SetDefaultLivesF _widgetref)
  (Default|SetDefaultTimerF _widgetref)
  (Default|ClearTimerF _widgetref))

(event EventBeginPlay
  (CallFunction|SetDefaultLivesF)
  (CallFunction|AddWidgetUIF)
  (CallFunction|SetDefaultLocationF))

(event Collision|EventActorBeginOverlap
  (params (OtherActor :type Actor%20Object%20Reference)))

(event EventTick
  (params (DeltaSeconds :type Float%20%28single-precision%29)))

(event Input|ActionEvents|InputActionFire
  (params (Key :type Key%20Structure :default "None"))
  (bind _camera (Variables|Default|GetCamera))
  (bind _returnvalue (Transformation|GetWorldRotation _camera))
  (:Pressed
    (Game|SpawnActorfromClass "/Game/Blueprints/Projectile/ProjectileBP.ProjectileBP_C" (Math|Transform|MakeTransform (+ (* (Math|Vector|GetForwardVector _returnvalue) 1e+02) (Transformation|GetWorldLocation _camera)) _returnvalue) "Undefined" 0 0)))

(event Input|AxisEvents|InputAxisMousePitch
  (params (AxisValue :type Float%20%28single-precision%29))
  (Pawn|Input|AddControllerPitchInput AxisValue))

(event Input|AxisEvents|InputAxisMouseYaw
  (params (AxisValue :type Float%20%28single-precision%29))
  (Pawn|Input|AddControllerYawInput AxisValue))

(event Input|AxisEvents|InputAxisMoveForward
  (params (AxisValue :type Float%20%28single-precision%29))
  (Pawn|Input|AddMovementInput (Math|Vector|GetForwardVector (Transformation|GetActorRotation)) AxisValue false))

(event Input|AxisEvents|InputAxisMoveRight
  (params (AxisValue :type Float%20%28single-precision%29))
  (Pawn|Input|AddMovementInput (Math|Vector|GetRightVector (Transformation|GetActorRotation)) AxisValue false))

(fn ConstructionScript)

(fn SetDefaultLivesF
  (bind _asuser_game_mode (Utilities|Casting|CastToUserGameMode (Game|GetGameMode)))
  (Variables|Default|SetLives (Variables|/Game/Blueprints/SuperClasses/UserGameMode.UserGameMode_C|GetDefaultLivesGiveToPlayer _asuser_game_mode)))

(fn AddWidgetUIF
  (bind _returnvalue (UserInterface|CreateWidget "/Game/Blueprints/Widgets/UserInterfaceW.UserInterfaceW_C"))
  (bind _output_get (Variables|Default|SetWidgetRef _returnvalue))
  (UserInterface|Viewport|AddtoViewport _output_get 0))

(fn ReducePlayerLivesF
  (if (== (Variables|Default|GetLives) 0)
    (CallFunction|PlayerFail)
    (else
      (Variables|Default|SetLives (- (Variables|Default|GetLives) 1))
      (Default|SetDefaultLivesF (Variables|Default|GetWidgetRef)))))

(fn TeleporttoStartF
  (Transformation|SetActorLocation (Variables|Default|GetPlayerLocation) false false))

(fn SetDefaultLocationF
  (Variables|Default|SetPlayerLocation (Transformation|GetActorLocation)))

(fn ResetPlayerValuesF
  (CallFunction|TeleporttoStartF))