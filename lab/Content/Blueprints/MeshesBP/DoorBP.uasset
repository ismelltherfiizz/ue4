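; Door actor that registers itself as DoorRef on UserGameMode at BeginPlay and slides open for a timed window.
; OpenDoor moves it, starts the countdown on the player character's widget, and sets a timer to call CloseDoor after the game mode's DefaultTimeGiveToPlayer.
; OpenCloseDoorF snaps the actor between two hard-coded world Y positions, with no interpolation, so it only suits one placement in the level.
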(event Custom|OpenDoor
  (CallFunction|OpenCloseDoorF true)
  (bind _asdefault_character (Utilities|Casting|CastToDefaultCharacter (Game|Player|GetPlayerPawn 0)))
  (Default|StartCountDownF (Variables|/Game/Blueprints/SuperClasses/DefaultCharacter.DefaultCharacter_C|GetWidgetRef _asdefault_character))
  (bind _asuser_game_mode (Utilities|Casting|CastToUserGameMode (Game|GetGameMode)))
  (Utilities|Time|SetTimerbyFunctionName 0 "CloseDoor" (Variables|/Game/Blueprints/SuperClasses/UserGameMode.UserGameMode_C|GetDefaultTimeGiveToPlayer _asuser_game_mode)))

(event Custom|CloseDoor
  (CallFunction|OpenCloseDoorF false))

(event Collision|EventActorBeginOverlap
  (params (OtherActor :type Actor%20Object%20Reference)))

(event EventTick
  (params (DeltaSeconds :type Float%20%28single-precision%29)))

(event EventBeginPlay
  (bind _asuser_game_mode (Utilities|Casting|CastToUserGameMode (Game|GetGameMode)))
  (Variables|/Game/Blueprints/SuperClasses/UserGameMode.UserGameMode_C|SetDoorRef _asuser_game_mode self))

(fn ConstructionScript)

(fn OpenCloseDoorF
  (params (is%20Open :type Boolean))
  (bind _returnvalue (Transformation|GetActorLocation))
  (bind _returnvalue_2 (Transformation|GetActorLocation))
  (if is%20Open
    (Transformation|SetActorLocation (Math|Vector|MakeVector (.x _returnvalue_2) -1.9e+03 (.z _returnvalue_2)) false false)
    (else
      (Transformation|SetActorLocation (Math|Vector|MakeVector (.x _returnvalue) -1774.0 (.z _returnvalue)) false false))))